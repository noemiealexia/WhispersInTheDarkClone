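; BP_MazeCell is a maze cell actor with four wall components, one for each cardinal direction.
; RemoveWall takes a direction and hides the matching wall, including its children, and disables its collision to open a passage.
; The cell has no active event or construction logic, so it changes only when RemoveWall is called.
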(fn `RemoveWall`
  (params (Direction :type Name))
  (bind _wall_north (`self.Wall_North`))
  (bind _wall_east (`self.Wall_East`))
  (bind _wall_south (`self.Wall_South`))
  (bind _wall_west (`self.Wall_West`))
  (switch `name` Direction
    (:`North`
      (`SceneComponent.SetVisibility` _wall_north false true)
      (`PrimitiveComponent.SetCollisionEnabled` _wall_north "NoCollision"))
    (:`South`
      (`SceneComponent.SetVisibility` _wall_south false true)
      (`PrimitiveComponent.SetCollisionEnabled` _wall_south "NoCollision"))
    (:`East`
      (`SceneComponent.SetVisibility` _wall_east false true)
      (`PrimitiveComponent.SetCollisionEnabled` _wall_east "NoCollision"))
    (:`West`
      (`SceneComponent.SetVisibility` _wall_west false true)
      (`PrimitiveComponent.SetCollisionEnabled` _wall_west "NoCollision"))))

(fn `UserConstructionScript`)