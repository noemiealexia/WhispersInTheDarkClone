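; Maze generator actor that spawns a grid of cell actors on BeginPlay, then carves passages between them.
; Delayed CarveMaze calls attempt a randomized depth-first backtracker, removing walls between unvisited neighbors via a cell stack.
; Each step re-pushes cell [0,0] and works from it, and rolls neighbor and direction separately, so carving cannot advance properly.
; Only the last spawned cell is attached; debug prints and a navmesh display aid testing.
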(event `self.ReceiveBeginPlay`
  (`KismetSystemLibrary.PrintString` "Maze Generation Started")
  ; X loop
  (for _index (range (`self.MazeSizeX`))
    (set `self.X_Index` _index)
    (bind _output_get (set `self.CurrentRow` (`|MakeArray` null :!type "/Game/Blueprints/BP_MazeCell Object Reference")))
    (`KismetArrayLibrary.Array_Clear` _output_get)
    ; Y Loop
    (for _index_2 (range (`self.MazeSizeY`))
      (set `self.Y_Index` _index_2)
      (bind _returnvalue (`|SpawnActorFromClass` (`self.CellClass`) (`KismetMathLibrary.MakeTransform` (`KismetMathLibrary.MakeVector` (* _index (`self.CellSize`)) (* _index_2 (`self.CellSize`)))) "Undefined" "MultiplyWithRoot" null false null))
      (bind _output_get_2 (set `self.CellActor` _returnvalue))
      (set `/Game/Blueprints/BP_MazeCell.GridPosition` (`KismetMathLibrary.MakeVector2D` (`KismetMathLibrary.Conv_IntToDouble` (`self.X_Index`)) (`KismetMathLibrary.Conv_IntToDouble` (`self.Y_Index`))) _output_get_2)
      (`KismetArrayLibrary.Array_Add` (`self.CurrentRow`) _output_get_2))
    (`KismetArrayLibrary.Array_Add` (`self.MazeGrid`) (make `/Game/Blueprints/MazeRowStruct` (`self.CurrentRow`))))
  (`self.K2_AttachToActor` (`self.CellActor`) self "None" "KeepRelative" "KeepRelative" "KeepRelative" true)
  (`KismetSystemLibrary.Delay` 0.2)
  (`self.CarveMazeStep`)
  (`KismetSystemLibrary.Delay` 0.2)
  (bind _output_get_3 (set `self.NavMeshLocation` (`NavigationSystemV1.K2_ProjectPointToNavigation` (`self.K2_GetActorLocation` (`self.CellActor`)))))
  (`KismetSystemLibrary.PrintString` "Nav Mesh Location:" true true (struct :`R` 1.0 :`G` 0.792013 :`A` 1.0) 10.0)
  (`KismetSystemLibrary.PrintString` (`KismetStringLibrary.Conv_VectorToString` _output_get_3) true true (struct :`R` 1.0 :`G` 0.792013 :`A` 1.0) 10.0)
  (`KismetSystemLibrary.ExecuteConsoleCommand` "Show Navigation" null))

(event `CarveMazeStep`
  (`KismetSystemLibrary.Delay` 0.5)
  (`self.CarveMaze`))

(fn `CarveMaze`
  (bind _mazestack (`self.MazeStack`))
  (bind _mazestack_2 (`self.MazeStack`))
  (bind _mazestack_3 (`self.MazeStack`))
  (bind _mazestack_4 (`self.MazeStack`))
  (bind _returnvalue (`KismetArrayLibrary.Array_Length` (`self.NeighborsList`)))
  (bind _returnvalue_2 (`KismetArrayLibrary.Array_Length` (`self.MazeStack`)))
  (bind (_cell _direction) (break `/Game/Blueprints/NeighborInfo` (`|GetArrayItem` (`self.NeighborsList`) (`KismetMathLibrary.RandomIntegerInRange` 0 (- (`KismetArrayLibrary.Array_Length` (`self.NeighborsList`)) 1)))))
  (bind _output_get (set `self.StartCell` (`|GetArrayItem` (`.Row_3_ED8903AE46A3FAE09109D7AA19966C97` (break `/Game/Blueprints/MazeRowStruct` (`|GetArrayItem` (`self.MazeGrid`)))))))
  (`/Engine/EditorBlueprintResources/StandardMacros.IsValid` _output_get
    (:`Is Valid`
      (set `/Game/Blueprints/BP_MazeCell.bVisited` true _output_get)
      (bind _output_get_2 (set `self.CurrentCell` _output_get))
      (`KismetArrayLibrary.Array_Add` (`self.MazeStack`) _output_get_2)
      (if (> (`KismetArrayLibrary.Array_Length` (`self.MazeStack`)) 0)
        (`KismetSystemLibrary.PrintString` "MazeStack Length:" true true (struct :`R` 0.315984 :`B` 1.0 :`A` 1.0) 10.0)
        (`KismetSystemLibrary.PrintString` (`KismetStringLibrary.Conv_IntToString` _returnvalue_2) true true (struct :`R` 0.288836 :`B` 1.0 :`A` 1.0) 10.0)
        (bind _output_get_3 (set `self.PeekedCell` (`|GetArrayItem` (`self.MazeStack`) (- _returnvalue_2 1))))
        (bind _output_get_4 (set `self.CurrentCell` _output_get_3))
        (bind (_gridposition_x _gridposition_y) (`KismetMathLibrary.BreakVector2D` (`/Game/Blueprints/BP_MazeCell.GridPosition` _output_get_4)))
        (bind _neighbors (`self.GetUnvisitedNeighbors` (`KismetMathLibrary.FTrunc` _gridposition_x) (`KismetMathLibrary.FTrunc` _gridposition_y)))
        (set `self.NeighborsList` _neighbors)
        (`KismetSystemLibrary.PrintString` (`KismetStringLibrary.Conv_IntToString` _returnvalue) true true (struct :`A` 1.0) 10.0)
        (if (> _returnvalue 0)
          (set `self.ChosenNeighbor` _cell)
          (bind _output_get_5 (set `self.Direction` _direction))
          (`/Game/Blueprints/BP_MazeCell.RemoveWall` (`self.CurrentCell`) _output_get_5)
          (bind _oppositedirection (`self.GetOppositeDirection` _output_get_5))
          (`/Engine/EditorBlueprintResources/StandardMacros.IsValid` (`self.ChosenNeighbor`)
            (:`Is Valid`
              (set `/Game/Blueprints/BP_MazeCell.bVisited` true (`self.ChosenNeighbor`))
              (`/Game/Blueprints/BP_MazeCell.RemoveWall` (`self.ChosenNeighbor`) _oppositedirection)
              (`KismetArrayLibrary.Array_Add` (`self.MazeStack`) (`self.ChosenNeighbor`))
              (set `self.CurrentCell` (`self.ChosenNeighbor`))
              (`self.CarveMazeStep`))
            (:`Is Not Valid`
              (`KismetSystemLibrary.PrintString` "ChosenNeighbor is not valid")
              (`KismetArrayLibrary.Array_Remove` _mazestack_3 (`KismetArrayLibrary.Array_LastIndex` _mazestack_3))
              (set `self.CurrentCell` (`|GetArrayItem` _mazestack_4 (`KismetArrayLibrary.Array_LastIndex` _mazestack_4)))
              (`self.CarveMazeStep`)))
          (else
            (`KismetSystemLibrary.PrintString` "No Neighbors found. Attempting backtrack..." true true (struct :`G` 0.5 :`B` 0.227826 :`A` 1.0) 10.0)
            (if (> (`KismetArrayLibrary.Array_Length` (`self.MazeStack`)) 0)
              (`KismetArrayLibrary.Array_Remove` _mazestack (`KismetArrayLibrary.Array_LastIndex` _mazestack))
              (bind _output_get_6 (set `self.CurrentCell` (`|GetArrayItem` _mazestack_2 (`KismetArrayLibrary.Array_LastIndex` _mazestack_2))))
              (`KismetSystemLibrary.PrintString` "Backtracking to:" true true (struct :`R` 1.0 :`B` 0.018576 :`A` 1.0) 10.0)
              (`KismetSystemLibrary.PrintString` (`KismetSystemLibrary.GetDisplayName` _output_get_6) true true (struct :`R` 1.0 :`B` 0.02448 :`A` 1.0) 10.0)
              (`self.CarveMazeStep`)
              (else
                (`KismetSystemLibrary.PrintString` "MazeStack is empty. Done!" true true (struct :`R` 1.0 :`G` 0.453125 :`B` 0.909977 :`A` 1.0) 10.0)))))
        (else
          (`KismetSystemLibrary.PrintString` "Maze Complete" true true (struct :`R` 1.0 :`B` 0.193642 :`A` 1.0) 10.0))))
    (:`Is Not Valid`
      (`KismetSystemLibrary.PrintString` "Start Cell Is None"))))

(fn `GetOppositeDirection`
  (params (Direction :type Name))
  (returns (OppositeDirection :type Name))
  (switch `name` Direction
    (:`North`
      (set `self.OppositeDirection` "South"))
    (:`South`
      (set `self.OppositeDirection` "North"))
    (:`East`
      (set `self.OppositeDirection` "West"))
    (:`West`
      (set `self.OppositeDirection` "East")))
  (return (`self.OppositeDirection`)))

(fn `GetUnvisitedNeighbors`
  (params (GridX :type Integer) (GridY :type Integer))
  (returns (Neighbors :type "Array of /Game/Blueprints/NeighborInfo Structure"))
  (bind _returnvalue (- (`local.GridX`) 1))
  (bind _returnvalue_2 (+ (`local.GridY`) 1))
  (bind _returnvalue_3 (- (`local.GridY`) 1))
  (bind _returnvalue_4 (+ (`local.GridX`) 1))
  (bind _output (`|GetArrayItem` (`.Row_3_ED8903AE46A3FAE09109D7AA19966C97` (break `/Game/Blueprints/MazeRowStruct` (`|GetArrayItem` (`self.MazeGrid`) (`local.GridX`)))) _returnvalue_2))
  (bind _output_2 (`|GetArrayItem` (`.Row_3_ED8903AE46A3FAE09109D7AA19966C97` (break `/Game/Blueprints/MazeRowStruct` (`|GetArrayItem` (`self.MazeGrid`) (`local.GridX`)))) _returnvalue_3))
  (bind _output_3 (`|GetArrayItem` (`.Row_3_ED8903AE46A3FAE09109D7AA19966C97` (break `/Game/Blueprints/MazeRowStruct` (`|GetArrayItem` (`self.MazeGrid`) _returnvalue))) (`local.GridY`)))
  (bind _output_4 (`|GetArrayItem` (`.Row_3_ED8903AE46A3FAE09109D7AA19966C97` (break `/Game/Blueprints/MazeRowStruct` (`|GetArrayItem` (`self.MazeGrid`) _returnvalue_4))) (`local.GridY`)))
  (set `self.FoundNeighbors` (`|MakeArray` (struct) :!type "/Game/Blueprints/NeighborInfo Structure"))
  (`|ExecutionSequence`
    (:`then_0`
      (if (< _returnvalue_2 (`self.MazeSizeY`))
        (bind _output_get (set `self.NorthCell` _output))
        (`/Engine/EditorBlueprintResources/StandardMacros.IsValid` _output_get
          (:`Is Valid`
            (if (not (`/Game/Blueprints/BP_MazeCell.bVisited` _output_get))
              (`KismetArrayLibrary.Array_Add` (`self.FoundNeighbors`) (make `/Game/Blueprints/NeighborInfo` _output "North"))
              (`KismetSystemLibrary.PrintString` "Added North to Neighbors" true true (struct :`R` 1.0 :`B` 0.154889 :`A` 1.0) 10.0)))
          (:`Is Not Valid`
            (`KismetSystemLibrary.PrintString` "North Cell Is Not Valid")))))
    (:`then_1`
      (if (>= _returnvalue_3 0)
        (if (not (`/Game/Blueprints/BP_MazeCell.bVisited` _output_2))
          (`KismetArrayLibrary.Array_Add` (`self.FoundNeighbors`) (make `/Game/Blueprints/NeighborInfo` _output_2 "South")))))
    (:`then_2`
      (if (< _returnvalue_4 (`self.MazeSizeX`))
        (if (not (`/Game/Blueprints/BP_MazeCell.bVisited` _output_4))
          (`KismetArrayLibrary.Array_Add` (`self.FoundNeighbors`) (make `/Game/Blueprints/NeighborInfo` _output_4 "East")))))
    (:`then_3`
      (if (>= _returnvalue 0)
        (if (not (`/Game/Blueprints/BP_MazeCell.bVisited` _output_3))
          (`KismetArrayLibrary.Array_Add` (`self.FoundNeighbors`) (make `/Game/Blueprints/NeighborInfo` _output_3 "West")))))
    (:`then_4`
      (`KismetSystemLibrary.PrintString` "FoundNeighbors array length:" true true (struct :`R` 1.0 :`B` 0.592295 :`A` 1.0) 15.0)
      (`KismetSystemLibrary.PrintString` (`KismetStringLibrary.Conv_IntToString` (`KismetArrayLibrary.Array_Length` (`self.FoundNeighbors`))) true true (struct :`R` 1.0 :`B` 0.50049 :`A` 1.0) 15.0)
      (return (`self.FoundNeighbors`)))))

(fn `UserConstructionScript`)